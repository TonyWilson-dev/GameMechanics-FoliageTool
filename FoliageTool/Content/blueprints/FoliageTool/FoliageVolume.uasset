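; Foliage volume actor that fills an area with copies of a given foliage actor's class.
; InitialiseFoliageVolume stores the settings, scales the cube or sphere component by Size, then calls Generate.
; Generate builds a jittered grid from Density × Size and component bounds at actor height, without clipping to the sphere.
; It spawns actors with random yaw and uniform scale, skipping unresolvable collisions; RandomOffset is stored but unused.
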(event `self.ReceiveBeginPlay`)

(fn `Generate`
  (bind _returnvalue (`KismetMathLibrary.RandomFloat`))
  (bind _foliagetype (`self.FoliageType`))
  (bind _spawn_transform_scale (`self.Spawn Transform Scale`))
  (bind (_origin _boxextent) (`KismetSystemLibrary.GetComponentBounds` (`self.foliage shape component`)))
  (bind (_origin_2 _boxextent_2) (`self.GetActorBounds` _foliagetype false false))
  (bind _returnvalue_2 (`KismetMathLibrary.Conv_Int64ToInt` (`KismetMathLibrary.Conv_IntToInt64` (`KismetMathLibrary.FTrunc` (* (`self.Density`) (`self.Size`))))))
  (for _index (range 1 (+ _returnvalue_2 1))
    (for _index_2 (range 1 (+ _returnvalue_2 1))
      (`KismetArrayLibrary.Array_Add` (`self.SpawnPoints`) (`KismetMathLibrary.MakeTransform` (`KismetMathLibrary.MakeVector` (+ (.x _origin) (* (/ _index_2 (`self.Size`)) (.x _boxextent) _returnvalue) (* (.x _boxextent_2) 2.0)) (+ (.y _origin) (* (/ _index (`self.Size`)) (.y _boxextent) _returnvalue) (* (.y _boxextent_2) 2.0)) (.z (.location (`self.GetTransform`))))))))
  (for _array_element (`self.SpawnPoints`)
    (`|SpawnActorFromClass` (`GameplayStatics.GetObjectClass` _foliagetype) (`KismetMathLibrary.MakeTransform` (.location _array_element) (`KismetMathLibrary.MakeRotator` (.roll (.rotation _array_element)) (.pitch (.rotation _array_element)) (`KismetMathLibrary.RandomFloatInRange` 0.0 (`self.RandomRotation`))) (`KismetMathLibrary.MakeVector` _spawn_transform_scale _spawn_transform_scale _spawn_transform_scale)) "AdjustIfPossibleButDontSpawnIfColliding" "OverrideRootScale" null null)))

(fn `Initialise Foliage Volume`
  (params (size :type "Float (double-precision)") (Density :type "Float (double-precision)") (Shape :type "/Game/blueprints/FoliageTool/FoliageShape Enum" :default "NewEnumerator0") (`Foliage Type` :type "Actor Object Reference (by ref)") (`Random Turning` :type "Float (double-precision) (by ref)") (`Actor Spawn Scale` :type "Float (double-precision) (by ref)") (`Random Offset` :type "Float (double-precision) (by ref)"))
  (returns (true :type Boolean))
  (set `self.Size` size)
  (set `self.Density` Density)
  (bind _output_get (set `self.VolumeShape` Shape))
  (switch `/Game/blueprints/FoliageTool/FoliageShape` _output_get
    (:`NewEnumerator0`
      (set `self.foliage shape component` (`self.Cube`))
      (`self.NewMacro_0`))
    (:`NewEnumerator1`
      (set `self.foliage shape component` (`self.Sphere1`))
      (`self.NewMacro`)))
  (set `self.FoliageType` `Foliage Type`)
  (set `self.RandomRotation` `Random Turning`)
  (set `self.Spawn Transform Scale` `Actor Spawn Scale`)
  (set `self.Random Offset` `Random Offset`)
  (`self.Generate`)
  (return true))

(fn `UserConstructionScript`)